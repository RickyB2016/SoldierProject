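; BP_deathbox is a kill volume that sets the MainCharacter's Health to zero when it overlaps the Box component.
; A random roll picks either a plain death or an explosive one.
; The explosive branch also sets ExplosionDeath and spawns an enlarged explosion emitter and mortar sound at the character's location.
; BeginPlay caches the player character, but the overlap logic works on the overlapping actor instead.
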(event OnComponentBeginOverlap(Box)
  (params (OverlappedComponent :type Primitive%20Component%20Object%20Reference) (OtherActor :type Actor%20Object%20Reference) (OtherComp :type Primitive%20Component%20Object%20Reference) (OtherBodyIndex :type Integer) (bFromSweep :type Boolean) (SweepResult :type Hit%20Result%20Structure%20%28by%20ref%29))
  (bind _asmain_character (Utilities|Casting|CastToMainCharacter OtherActor))
  (bind _output_get (Variables|Default|SetRandomDeath (Math|Random|RandomIntegerinRange 0 1)))
  (switch int _output_get
    (:0
      (Variables|/Game/SOLDIER/Characters/MainCharacter.MainCharacter_C|SetHealth _asmain_character 0.0))
    (:1
      (Variables|/Game/SOLDIER/Characters/MainCharacter.MainCharacter_C|SetExplosionDeath _asmain_character true)
      (Variables|/Game/SOLDIER/Characters/MainCharacter.MainCharacter_C|SetHealth _asmain_character 0.0)
      (bind _returnvalue (Effects|SpawnEmitteratLocation "/Game/StarterContent/Particles/P_Explosion.P_Explosion" (Transformation|GetActorLocation _asmain_character)))
      (Transformation|SetRelativeScale3D _returnvalue "30.000000,30.000000,30.000000")
      (Audio|PlaySoundatLocation "/Game/SOLDIER/SFX/Mortor/SC_MortorExplosion.SC_MortorExplosion" (Transformation|GetActorLocation _asmain_character) "0, 0, 0" 1.0))))

(event EventBeginPlay
  (bind _asmain_character (Utilities|Casting|CastToMainCharacter (Game|Player|GetPlayerPawn 0)))
  (Variables|Default|SetCharacter _asmain_character))

(event Collision|EventActorBeginOverlap
  (params (OtherActor :type Actor%20Object%20Reference)))

(event EventTick
  (params (DeltaSeconds :type Float%20%28single-precision%29)))

(fn ConstructionScript)