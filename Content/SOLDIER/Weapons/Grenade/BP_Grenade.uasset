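; Grenade actor that plays surface-specific landing sounds and provides an explosion that can kill the player.
; Tick traces just below the mesh until a wood, mud, grass or gravel physical surface latches Landed.
; Explode, not called within this file, radially impulses sphere-traced objects and, per hit, checks overlap volumes to kill or camera-shake the player.
; It then spawns particles, plays one of two random sounds and destroys itself.
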(event EventBeginPlay
  (bind _asmain_character (Utilities|Casting|CastToMainCharacter (Game|Player|GetPlayerPawn 0)))
  (Variables|Default|SetCharacter _asmain_character))

(event EventTick
  (params (DeltaSeconds :type Float%20%28single-precision%29))
  (bind _grenademesh (Variables|Default|GetGrenadeMesh))
  (bind _returnvalue (Transformation|GetWorldLocation _grenademesh))
  (if (not (Variables|Default|GetLanded))
    (bind _outhit (Collision|LineTraceByChannel _returnvalue (- _returnvalue "0, 0,10.000000") "TraceTypeQuery1" false 0 "None"))
    (switch Utilities|FlowControl|Switch|SwitchonEPhysicalSurface (Variables|/Script/Engine.PhysicalMaterial|GetSurfaceType (.PhysMat (Collision|BreakHitResult _outhit)))
      (:SurfaceType1
        (Audio|PlaySoundatLocation "/Game/SOLDIER/SFX/Grenade/MSGA_Soldier_SD_Grenade_Hit_Wood_V1.MSGA_Soldier_SD_Grenade_Hit_Wood_V1" (.ImpactPoint (Collision|BreakHitResult _outhit)) :!label _label)
        (Development|PrintString "wood"))
      (:SurfaceType2
        (goto _label))
      (:SurfaceType3
        (Audio|PlaySoundatLocation "/Game/SOLDIER/SFX/Grenade/MSGA_Soldier_SD_Grenade_Hit_Mud_V1.MSGA_Soldier_SD_Grenade_Hit_Mud_V1" (.ImpactPoint (Collision|BreakHitResult _outhit)))
        (Development|PrintString "mud"))
      (:SurfaceType4
        (Audio|PlaySoundatLocation "/Game/SOLDIER/SFX/Grenade/MSGA_Soldier_SD_Grenade_Hit_V1.MSGA_Soldier_SD_Grenade_Hit_V1" (.ImpactPoint (Collision|BreakHitResult _outhit)) :!label _label_2)
        (Development|PrintString "grass"))
      (:SurfaceType5
        (goto _label_2)))
    (bind _output_get (Variables|Default|SetLanded true))
    (Development|PrintString (Utilities|String|ToString(Boolean) _output_get))))

(fn ConstructionScript)

(fn Explode
  (bind _character (Variables|Default|GetCharacter))
  (bind _grenademesh (Variables|Default|GetGrenadeMesh))
  (bind _returnvalue (Transformation|GetWorldLocation _grenademesh))
  (bind (_outhits _returnvalue_2) (Collision|MultiSphereTraceForObjects _returnvalue _returnvalue 1e+03 (Utilities|Array|MakeArray "ObjectTypeQuery4" "ObjectTypeQuery2" "ObjectTypeQuery3") false 0 "None"))
  (if _returnvalue_2
    _
    (else
      _))
  (for _array_element _outhits
    ;[1 1 1] launch physics objects
    (Physics|AddRadialImpulse (.HitComponent (Collision|BreakHitResult _array_element)) (Transformation|GetWorldLocation (Variables|Default|GetGrenadeMesh)) 9e+02 2e+05 "RIF_Constant" false)
    (if (Collision|IsOverlappingActor (Variables|Default|GetDeathBox) (Variables|Default|GetCharacter) :!class /Script/Engine.PrimitiveComponent)
      (Development|PrintString "death")
      (Variables|/Game/SOLDIER/Characters/MainCharacter.MainCharacter_C|SetExplosionDeath _character true)
      (Variables|/Game/SOLDIER/Characters/MainCharacter.MainCharacter_C|SetHealth _character 0.0)
      (elif (Collision|IsOverlappingActor (Variables|Default|GetCameraShake) (Variables|Default|GetCharacter) :!class /Script/Engine.PrimitiveComponent)
        (Development|PrintString "shake")
        (Class|PlayerController|ClientPlayCameraShake (Game|GetPlayerController 0) "/Game/SOLDIER/Post-Processing/CameraShake/Explosion/BP_Explosion_CameraShake.BP_Explosion_CameraShake_C" 22.0 "CameraLocal" "0, 0, 0"))))
  (bind _returnvalue_3 (Effects|SpawnEmitteratLocation "/Game/UE4_Starter_Content/Particles/P_Explosion.P_Explosion" _returnvalue))
  (Transformation|SetRelativeScale3D _returnvalue_3 "10.000000,10.000000,10.000000")
  (switch int (Math|Random|RandomIntegerinRange 0 1)
    (:0
      (Audio|PlaySoundatLocation "/Game/SOLDIER/SFX/Grenade/MSGA_Soldier_SD_Grenade_Explosion_Long_V1_1.MSGA_Soldier_SD_Grenade_Explosion_Long_V1_1" _returnvalue "0, 0, 0" 0.5))
    (:1
      (Audio|PlaySoundatLocation "/Game/SOLDIER/SFX/Grenade/MSGA_Soldier_SD_Grenade_Explosion_Short_V1.MSGA_Soldier_SD_Grenade_Explosion_Short_V1" _returnvalue "0, 0, 0" 0.5)))
  (Actor|DestroyActor))

(fn LandingMaterial)