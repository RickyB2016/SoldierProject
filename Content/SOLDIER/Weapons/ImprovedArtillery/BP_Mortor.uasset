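; BP_Mortor is an artillery strike actor that plays an incoming whistle, then may explode at its location.
; After fixed delays, a random roll triggers one of two explosion sounds and a scaled-up emitter on only two of its outcomes.
; Hit box overlap kills the player character, while the outer collision gives camera shake.
; The cycle repeats only after a kill or shake; other outcomes end it.
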(event EventBeginPlay
  (bind _asmain_character (Utilities|Casting|CastToMainCharacter (Game|Player|GetPlayerPawn 0) :!label _label))
  (Variables|Default|SetCharacter _asmain_character)
  (bind _output_get (Variables|Default|SetRandomDelay 3))
  (Utilities|FlowControl|Delay (Math|Conversions|ToFloat(Integer) _output_get))
  (Audio|Components|Audio|Play (Variables|Default|GetLaunchWhistle_Audio) 0.0)
  (Utilities|FlowControl|Delay 8.5)
  (bind _output_get_2 (Variables|Default|SetRandomExplosion (Math|Random|RandomIntegerinRange 0 60)))
  (switch int _output_get_2
    (:0
      (Audio|Components|Audio|Play (Variables|Default|GetExplosion_AudioV2) 0.0))
    (:1
      (Audio|Components|Audio|Play (Variables|Default|GetExplosion_Audio) 0.0)))
  (bind _returnvalue (Effects|SpawnEmitteratLocation "/Game/UE4_Starter_Content/Particles/P_Explosion.P_Explosion" (Transformation|GetActorLocation)))
  (Transformation|SetRelativeScale3D _returnvalue "60.000000,60.000000,60.000000")
  (if (Collision|IsOverlappingActor (Variables|Default|GetArtillery_HitBox) (Variables|Default|GetCharacter) :!class /Script/Engine.PrimitiveComponent)
    (Utilities|FlowControl|Sequence
      (:then_0
        (Variables|/Game/SOLDIER/Characters/MainCharacter.MainCharacter_C|SetExplosionDeath (Variables|Default|GetCharacter) true)
        (Components|Activation|Activate (Variables|/Game/SOLDIER/Characters/MainCharacter.MainCharacter_C|GetMainCamera (Variables|Default|GetCharacter)) false)
        (Components|Activation|Deactivate (Variables|/Game/SOLDIER/Characters/MainCharacter.MainCharacter_C|GetTransition_Camera (Variables|Default|GetCharacter)))
        (Variables|/Game/SOLDIER/Characters/MainCharacter.MainCharacter_C|SetHealth (Variables|Default|GetCharacter) 0.0)
        (Utilities|FlowControl|Delay 1.5)
        (goto _label)))
    (elif (Collision|IsOverlappingActor (Variables|Default|GetCameraShakeCollision) (Variables|Default|GetCharacter) :!class /Script/Engine.PrimitiveComponent)
      (Class|PlayerController|ClientPlayCameraShake (Game|GetPlayerController 0) "/Game/SOLDIER/Post-Processing/CameraShake/Explosion/BP_Explosion_CameraShake.BP_Explosion_CameraShake_C" 1e+01 "CameraLocal" "0, 0, 0")
      (goto _label))))

(fn ConstructionScript)