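; BP_ArtilleryLVL3 is an artillery strike actor that plays a whistle sound, then spawns a large explosion at its location.
; On BeginPlay it casts the player pawn to both MainCharacter and AI_Character, then waits a random delay and picks one of two whistles.
; Hitbox overlap kills the player or flags the AI reference's explosion death; an outer volume shakes the camera.
; The cycle repeats only when the player is caught in either volume.
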(event EventBeginPlay
  (bind _asmain_character (Utilities|Casting|CastToMainCharacter (Game|Player|GetPlayerPawn 0) :!label _label))
  (Variables|Default|SetCharacter _asmain_character)
  (bind _asai_character (Utilities|Casting|CastToAI_Character (Game|Player|GetPlayerPawn 0)))
  (Variables|Default|SetAIEnemy _asai_character)
  (bind _output_get (Variables|Default|SetRandomDelay (Math|Random|RandomIntegerinRange 0 15)))
  (Utilities|FlowControl|Delay (Math|Conversions|ToFloat(Integer) _output_get))
  (bind _output_get_2 (Variables|Default|SetRandomExplosion (Math|Random|RandomIntegerinRange 0 1)))
  (switch int _output_get_2
    (:0
      (Audio|Components|Audio|Play (Variables|Default|GetWhistelLand_AudioV2) 0.0))
    (:1
      (Audio|Components|Audio|Play (Variables|Default|GetWhistleLand_Audio) 0.0)))
  (Utilities|FlowControl|Delay 1.3)
  (bind _returnvalue (Effects|SpawnEmitteratLocation "/Game/UE4_Starter_Content/Particles/P_Explosion.P_Explosion" (Transformation|GetActorLocation)))
  (Transformation|SetRelativeScale3D _returnvalue "80.000000,80.000000,80.000000")
  (Utilities|FlowControl|Sequence
    (:then_0
      (if (Collision|IsOverlappingActor (Variables|Default|GetArtillery_HitBox) (Variables|Default|GetCharacter) :!class /Script/Engine.PrimitiveComponent)
        (Variables|/Game/SOLDIER/Characters/MainCharacter.MainCharacter_C|SetExplosionDeath (Variables|Default|GetCharacter) true)
        (Variables|/Game/SOLDIER/Characters/MainCharacter.MainCharacter_C|SetHealth (Variables|Default|GetCharacter) 0.0)
        (goto _label)
        (elif (Collision|IsOverlappingActor (Variables|Default|GetCameraShakeCollision) (Variables|Default|GetCharacter) :!class /Script/Engine.PrimitiveComponent)
          (Class|PlayerController|ClientPlayCameraShake (Game|GetPlayerController 0) "/Game/SOLDIER/Post-Processing/CameraShake/Explosion/BP_Explosion_CameraShake.BP_Explosion_CameraShake_C" 1e+01 "CameraLocal" "0, 0, 0")
          (goto _label))))
    (:then_1
      (if (Collision|IsOverlappingActor (Variables|Default|GetArtillery_HitBox) (Variables|Default|GetAIEnemy) :!class /Script/Engine.PrimitiveComponent)
        (Variables|/Game/SOLDIER/AI/AI_Character.AI_Character_C|SetExplosionDeath (Variables|Default|GetAIEnemy) true)))))

(event Collision|EventActorBeginOverlap
  (params (OtherActor :type Actor%20Object%20Reference)))

(event EventTick
  (params (DeltaSeconds :type Float%20%28single-precision%29)))

(fn ConstructionScript)